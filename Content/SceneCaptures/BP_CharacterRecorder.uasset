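; Scene-capture character stand-in that mirrors equipped armor and weapons on its own skeletal mesh.
; On BeginPlay it passes itself to the player's ThirdPersonCharacterIgnore, and exposes EquipItem and UnEquipItem events.
; AttachItem replaces the slot's actor with a new spawn, snapped to the socket from its armor or weapon info, with collision disabled.
; Left-hand slots accept weapons or armor; UnattachItem destroys the slot's actor.
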(event `self.ReceiveBeginPlay`
  (bind _asthird_person_character_ignore (cast `/Game/ThirdPersonBP/Blueprints/ThirdPersonCharacterIgnore` (`GameplayStatics.GetPlayerCharacter` 0)))
  (message `/Game/Interactables/BPI_RecorderComm.PassReference` _asthird_person_character_ignore self))

(event `/Game/Interactables/BPI_RecorderComm.EquipItem`
  (params (ItemInfo :type "/Game/Interactables/FitemInfo Structure"))
  (`self.AttachItem` ItemInfo))

(event `/Game/Interactables/BPI_RecorderComm.UnEquipItem`
  (params (ItemInfo :type "/Game/Interactables/FitemInfo Structure"))
  (`self.UnattachItem` ItemInfo))

(fn `AttachItem`
  (params (ItemInfo :type "/Game/Interactables/FitemInfo Structure"))
  (bind ((`itemClass_13_99493ACF4E749688B76FD0A3C848D836` _itemclass) (`ItemSlot_20_53CE742C40F9A64BD794C9960A402A17` _itemslot)) (break `/Game/Interactables/FitemInfo` ItemInfo))
  (switch `/Game/Interactables/ESlotType` _itemslot
    (:`NewEnumerator1`
      (`/Engine/EditorBlueprintResources/StandardMacros.IsValid` (`self.Head Item`)
        (:`Is Valid`
          (`self.K2_DestroyActor` (`self.Head Item`)))
        (:`Is Not Valid`
          _))
      (bind _returnvalue (`|SpawnActorFromClass` _itemclass (`self.GetTransform`) "AlwaysSpawn" "OverrideRootScale" null null))
      (bind _output_get (set `self.Head Item` _returnvalue))
      (bind _asbp_base_armor (cast `/Game/Interactables/Armor/BP_BaseArmor` _output_get))
      (`self.K2_AttachToComponent` _asbp_base_armor (`self.SkeletalMesh`) (`.AttachPoint_5_3C313C0F454E5170FA03E1B1444B6C66` (break `/Game/Interactables/Armor/FArmorInfo` (`/Game/Interactables/Armor/BP_BaseArmor.ArmorInfo` _asbp_base_armor))) "SnapToTarget" "SnapToTarget" "SnapToTarget" true)
      (`self.SetActorEnableCollision` _asbp_base_armor false))
    (:`NewEnumerator2`
      (`/Engine/EditorBlueprintResources/StandardMacros.IsValid` (`self.Torso Item`)
        (:`Is Valid`
          (`self.K2_DestroyActor` (`self.Torso Item`)))
        (:`Is Not Valid`
          _))
      (bind _returnvalue_2 (`|SpawnActorFromClass` _itemclass (`self.GetTransform`) "AlwaysSpawn" "OverrideRootScale" null null))
      (bind _output_get_2 (set `self.Torso Item` _returnvalue_2))
      (bind _asbp_base_armor_2 (cast `/Game/Interactables/Armor/BP_BaseArmor` _output_get_2))
      (`self.K2_AttachToComponent` _asbp_base_armor_2 (`self.SkeletalMesh`) (`.AttachPoint_5_3C313C0F454E5170FA03E1B1444B6C66` (break `/Game/Interactables/Armor/FArmorInfo` (`/Game/Interactables/Armor/BP_BaseArmor.ArmorInfo` _asbp_base_armor_2))) "SnapToTarget" "SnapToTarget" "SnapToTarget" true)
      (`self.SetActorEnableCollision` _asbp_base_armor_2 false))
    (:`NewEnumerator3`
      (`/Engine/EditorBlueprintResources/StandardMacros.IsValid` (`self.Arms Item`)
        (:`Is Valid`
          (`self.K2_DestroyActor` (`self.Arms Item`)))
        (:`Is Not Valid`
          _))
      (bind _returnvalue_3 (`|SpawnActorFromClass` _itemclass (`self.GetTransform`) "AlwaysSpawn" "OverrideRootScale" null null))
      (bind _output_get_3 (set `self.Arms Item` _returnvalue_3))
      (bind _asbp_base_armor_3 (cast `/Game/Interactables/Armor/BP_BaseArmor` _output_get_3))
      (`self.K2_AttachToComponent` _asbp_base_armor_3 (`self.SkeletalMesh`) (`.AttachPoint_5_3C313C0F454E5170FA03E1B1444B6C66` (break `/Game/Interactables/Armor/FArmorInfo` (`/Game/Interactables/Armor/BP_BaseArmor.ArmorInfo` _asbp_base_armor_3))) "SnapToTarget" "SnapToTarget" "SnapToTarget" true)
      (`self.SetActorEnableCollision` _asbp_base_armor_3 false))
    (:`NewEnumerator4`
      (`/Engine/EditorBlueprintResources/StandardMacros.IsValid` (`self.Legs Item`)
        (:`Is Valid`
          (`self.K2_DestroyActor` (`self.Legs Item`)))
        (:`Is Not Valid`
          _))
      (bind _returnvalue_4 (`|SpawnActorFromClass` _itemclass (`self.GetTransform`) "AlwaysSpawn" "OverrideRootScale" null null))
      (bind _output_get_4 (set `self.Legs Item` _returnvalue_4))
      (bind _asbp_base_armor_4 (cast `/Game/Interactables/Armor/BP_BaseArmor` _output_get_4))
      (`self.K2_AttachToComponent` _asbp_base_armor_4 (`self.SkeletalMesh`) (`.AttachPoint_5_3C313C0F454E5170FA03E1B1444B6C66` (break `/Game/Interactables/Armor/FArmorInfo` (`/Game/Interactables/Armor/BP_BaseArmor.ArmorInfo` _asbp_base_armor_4))) "SnapToTarget" "SnapToTarget" "SnapToTarget" true)
      (`self.SetActorEnableCollision` _asbp_base_armor_4 false))
    (:`NewEnumerator5`
      (`/Engine/EditorBlueprintResources/StandardMacros.IsValid` (`self.Feet Item`)
        (:`Is Valid`
          (`self.K2_DestroyActor` (`self.Feet Item`)))
        (:`Is Not Valid`
          _))
      (bind _returnvalue_5 (`|SpawnActorFromClass` _itemclass (`self.GetTransform`) "AlwaysSpawn" "OverrideRootScale" null null))
      (bind _output_get_5 (set `self.Feet Item` _returnvalue_5))
      (bind _asbp_base_armor_5 (cast `/Game/Interactables/Armor/BP_BaseArmor` _output_get_5))
      (`self.K2_AttachToComponent` _asbp_base_armor_5 (`self.SkeletalMesh`) (`.AttachPoint_5_3C313C0F454E5170FA03E1B1444B6C66` (break `/Game/Interactables/Armor/FArmorInfo` (`/Game/Interactables/Armor/BP_BaseArmor.ArmorInfo` _asbp_base_armor_5))) "SnapToTarget" "SnapToTarget" "SnapToTarget" true)
      (`self.SetActorEnableCollision` _asbp_base_armor_5 false))
    (:`NewEnumerator6`
      (`/Engine/EditorBlueprintResources/StandardMacros.IsValid` (`self.PRH_Item`)
        (:`Is Valid`
          (`self.K2_DestroyActor` (`self.PRH_Item`)))
        (:`Is Not Valid`
          _))
      (bind _returnvalue_6 (`|SpawnActorFromClass` _itemclass (`self.GetTransform`) "AlwaysSpawn" "OverrideRootScale" null null))
      (bind _output_get_6 (set `self.PRH_Item` _returnvalue_6))
      (bind _asbp_base_weapon (cast `/Game/Interactables/Weapons/BP_BaseWeapon` _output_get_6))
      (`self.K2_AttachToComponent` _asbp_base_weapon (`self.SkeletalMesh`) (`.PrimaryRightHand_15_D27C505643EC79E4EFC75D9E1EF9FD12` (break `/Game/Interactables/Weapons/FWeaponInfo` (`/Game/Interactables/Weapons/BP_BaseWeapon.WeaponInfo` _asbp_base_weapon))) "SnapToTarget" "SnapToTarget" "SnapToTarget" true)
      (`self.SetActorEnableCollision` _asbp_base_weapon false))
    (:`NewEnumerator7`
      (`/Engine/EditorBlueprintResources/StandardMacros.IsValid` (`self.PLH_Item`)
        (:`Is Valid`
          (`self.K2_DestroyActor` (`self.PLH_Item`)))
        (:`Is Not Valid`
          _))
      (bind _returnvalue_7 (`|SpawnActorFromClass` _itemclass (`self.GetTransform`) "AlwaysSpawn" "OverrideRootScale" null null))
      (bind _output_get_7 (set `self.PLH_Item` _returnvalue_7))
      (bind _asbp_base_weapon_2 (cast `/Game/Interactables/Weapons/BP_BaseWeapon` _output_get_7)
        (:`then`
          (`self.K2_AttachToComponent` _asbp_base_weapon_2 (`self.SkeletalMesh`) (`.PrinaryLeftHand_19_6D4A65BD48AC8A731393D2B3C4841608` (break `/Game/Interactables/Weapons/FWeaponInfo` (`/Game/Interactables/Weapons/BP_BaseWeapon.WeaponInfo` _asbp_base_weapon_2))) "SnapToTarget" "SnapToTarget" "SnapToTarget" true)
          (`self.SetActorEnableCollision` _asbp_base_weapon_2 false))
        (:`CastFailed`
          (bind _asbp_base_armor_6 (cast `/Game/Interactables/Armor/BP_BaseArmor` _output_get_7))
          (`self.K2_AttachToComponent` _asbp_base_armor_6 (`self.SkeletalMesh`) (`.AttachPoint_5_3C313C0F454E5170FA03E1B1444B6C66` (break `/Game/Interactables/Armor/FArmorInfo` (`/Game/Interactables/Armor/BP_BaseArmor.ArmorInfo` _asbp_base_armor_6))) "SnapToTarget" "SnapToTarget" "SnapToTarget" true)
          (`self.SetActorEnableCollision` _asbp_base_armor_6 false))))
    (:`NewEnumerator8`
      (`/Engine/EditorBlueprintResources/StandardMacros.IsValid` (`self.SRH_Item`)
        (:`Is Valid`
          (`self.K2_DestroyActor` (`self.SRH_Item`)))
        (:`Is Not Valid`
          _))
      (bind _returnvalue_8 (`|SpawnActorFromClass` _itemclass (`self.GetTransform`) "AlwaysSpawn" "OverrideRootScale" null null))
      (bind _output_get_8 (set `self.SRH_Item` _returnvalue_8))
      (bind _asbp_base_weapon_3 (cast `/Game/Interactables/Weapons/BP_BaseWeapon` _output_get_8))
      (`self.K2_AttachToComponent` _asbp_base_weapon_3 (`self.SkeletalMesh`) (`.SecondaryRightHand_20_F42B210E48D2A21B51A334AAB2ABA509` (break `/Game/Interactables/Weapons/FWeaponInfo` (`/Game/Interactables/Weapons/BP_BaseWeapon.WeaponInfo` _asbp_base_weapon_3))) "SnapToTarget" "SnapToTarget" "SnapToTarget" true)
      (`self.SetActorEnableCollision` _asbp_base_weapon_3 false))
    (:`NewEnumerator9`
      (`/Engine/EditorBlueprintResources/StandardMacros.IsValid` (`self.SLH_Item`)
        (:`Is Valid`
          (`self.K2_DestroyActor` (`self.SLH_Item`)))
        (:`Is Not Valid`
          _))
      (bind _returnvalue_9 (`|SpawnActorFromClass` _itemclass (`self.GetTransform`) "AlwaysSpawn" "OverrideRootScale" null null))
      (bind _output_get_9 (set `self.SLH_Item` _returnvalue_9))
      (bind _asbp_base_weapon_4 (cast `/Game/Interactables/Weapons/BP_BaseWeapon` _output_get_9)
        (:`then`
          (`self.K2_AttachToComponent` _asbp_base_weapon_4 (`self.SkeletalMesh`) (`.SecondaryLeftHand_21_67FA69C44AE9ABFEE88E8D9546DAC211` (break `/Game/Interactables/Weapons/FWeaponInfo` (`/Game/Interactables/Weapons/BP_BaseWeapon.WeaponInfo` _asbp_base_weapon_4))) "SnapToTarget" "SnapToTarget" "SnapToTarget" true)
          (`self.SetActorEnableCollision` _asbp_base_weapon_4 false))
        (:`CastFailed`
          (bind _asbp_base_armor_7 (cast `/Game/Interactables/Armor/BP_BaseArmor` _output_get_9))
          (`self.K2_AttachToComponent` _asbp_base_armor_7 (`self.SkeletalMesh`) (`.AttachPoint_5_3C313C0F454E5170FA03E1B1444B6C66` (break `/Game/Interactables/Armor/FArmorInfo` (`/Game/Interactables/Armor/BP_BaseArmor.ArmorInfo` _asbp_base_armor_7))) "SnapToTarget" "SnapToTarget" "SnapToTarget" true)
          (`self.SetActorEnableCollision` _asbp_base_armor_7 false))))))

(fn `UnattachItem`
  (params (ItemInfo :type "/Game/Interactables/FitemInfo Structure"))
  (switch `/Game/Interactables/ESlotType` (`.ItemSlot_20_53CE742C40F9A64BD794C9960A402A17` (break `/Game/Interactables/FitemInfo` ItemInfo))
    (:`NewEnumerator1`
      (`self.K2_DestroyActor` (`self.Head Item`)))
    (:`NewEnumerator2`
      (`self.K2_DestroyActor` (`self.Torso Item`)))
    (:`NewEnumerator3`
      (`self.K2_DestroyActor` (`self.Arms Item`)))
    (:`NewEnumerator4`
      (`self.K2_DestroyActor` (`self.Legs Item`)))
    (:`NewEnumerator5`
      (`self.K2_DestroyActor` (`self.Feet Item`)))
    (:`NewEnumerator6`
      (`self.K2_DestroyActor` (`self.PRH_Item`)))
    (:`NewEnumerator7`
      (`self.K2_DestroyActor` (`self.PLH_Item`)))
    (:`NewEnumerator8`
      (`self.K2_DestroyActor` (`self.SRH_Item`)))
    (:`NewEnumerator9`
      (`self.K2_DestroyActor` (`self.SLH_Item`)))))

(fn `UserConstructionScript`)