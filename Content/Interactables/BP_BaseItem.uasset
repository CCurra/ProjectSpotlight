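; BP_BaseItem is a base pickup item that an interacting actor can collect into its inventory.
; On Interaction, it checks that the instigator has inventory space, passes it the ItemInfo struct via PickUpMessage, then destroys itself.
; The construction script rebuilds ItemInfo with the actor's own class filled in, keeping the other fields, so the stored data records which class the item came from.
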(event `/Game/Interactables/BPI_Interact.interaction**`
  (params (Instagator :type "/Game/ThirdPersonBP/Blueprints/ThirdPersonCharacter Object Reference"))
  (if (`/Game/ThirdPersonBP/Blueprints/ThirdPersonCharacter.HasSpaceInInventory` Instagator)
    (message `/Game/Interactables/BPI_Interact.PickUp` Instagator (`self.ItemInfo`))
    (`self.K2_DestroyActor`)))

(fn `UserConstructionScript`
  (bind (_iteminfo_itemtype _iteminfo_itemname _iteminfo_itemimage _iteminfo_itemclass _iteminfo_itemindex _iteminfo_itemslot _iteminfo_itemvalue) (break `/Game/Interactables/FitemInfo` (`self.ItemInfo`)))
  (`parent.UserConstructionScript`)
  (set `self.ItemInfo` (make `/Game/Interactables/FitemInfo` _iteminfo_itemtype _iteminfo_itemname _iteminfo_itemimage (`GameplayStatics.GetObjectClass` self) _iteminfo_itemindex _iteminfo_itemslot _iteminfo_itemvalue)))