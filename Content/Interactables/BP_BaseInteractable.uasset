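; Base interactable actor that registers itself with a ThirdPersonCharacter on overlap and supports outline-style highlighting.
; Begin overlap on InteractableArea sends the character a register message, while end overlap on InteractableMesh, a different component, sends the unregister message.
; SetHighlight toggles the mesh's custom depth rendering, but only while the given player has no weapon attached, so the current state otherwise stays unchanged.
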(event `self.InteractableArea.OnComponentBeginOverlap`
  (params (OverlappedComponent :type "PrimitiveComponent Object Reference") (OtherActor :type "Actor Object Reference") (OtherComp :type "PrimitiveComponent Object Reference") (OtherBodyIndex :type Integer) (bFromSweep :type Boolean) (SweepResult :type "HitResult Structure (by ref)"))
  (bind _asthird_person_character (cast `/Game/ThirdPersonBP/Blueprints/ThirdPersonCharacter` OtherActor))
  (message `/Game/Interactables/BPI_Interact.RegisterInteractable` _asthird_person_character self))

(event `self.InteractableMesh.OnComponentEndOverlap`
  (params (OverlappedComponent :type "PrimitiveComponent Object Reference") (OtherActor :type "Actor Object Reference") (OtherComp :type "PrimitiveComponent Object Reference") (OtherBodyIndex :type Integer))
  (bind _asthird_person_character (cast `/Game/ThirdPersonBP/Blueprints/ThirdPersonCharacter` OtherActor))
  (message `/Game/Interactables/BPI_Interact.UnregisteredInteractable` _asthird_person_character self))

(fn `SetHighlight`
  (params (`highlight?` :type Boolean) (Player :type "/Game/ThirdPersonBP/Blueprints/ThirdPersonCharacter Object Reference"))
  (if (not (`/Game/ThirdPersonBP/Blueprints/ThirdPersonCharacter.HasWeaponAttached` Player))
    (`PrimitiveComponent.SetRenderCustomDepth` (`self.InteractableMesh`) `highlight?`)))

(fn `UserConstructionScript`)